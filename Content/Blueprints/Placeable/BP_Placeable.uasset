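; BP_Placeable is a placeable prop that takes on a random primitive shape and animates in when it spawns.
; The construction script randomly assigns a cone, sphere or cylinder to its static mesh.
; On BeginPlay the IntroAnim timeline drives the mesh's relative location along a fall curve and its scale along a scale curve.
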(event `self.ReceiveBeginPlay`
  (bind _staticmesh (`self.StaticMesh`))
  (bind (_direction _fall _scaleanim) (`Timeline|Intro Anim` :!via `PlayFromStart`)
    (:`Update`
      (`SceneComponent.K2_SetRelativeLocation` _staticmesh _fall false true)
      (`SceneComponent.SetRelativeScale3D` _staticmesh _scaleanim))))

(fn `UserConstructionScript`
  (switch `int` (`KismetMathLibrary.RandomInteger` 3)
    (:`0`
      (`StaticMeshComponent.SetStaticMesh` (`self.StaticMesh`) "/Engine/BasicShapes/Cone.Cone"))
    (:`1`
      (`StaticMeshComponent.SetStaticMesh` (`self.StaticMesh`) "/Engine/BasicShapes/Sphere.Sphere"))
    (:`2`
      (`StaticMeshComponent.SetStaticMesh` (`self.StaticMesh`) "/Engine/BasicShapes/Cylinder.Cylinder"))))